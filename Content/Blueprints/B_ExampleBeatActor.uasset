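; Example actor that exercises the UniversalBeatSubsystem for music playback and beat-timed input.
; On BeginPlay it sets the BPM, enables sixteenth-note beat broadcasting, plays the base song, then binds song-started and track-started events that print debug text.
; The IA_Tap input action queries beat timing by label and prints the result.
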(event Custom|OnSongStarted_Event
  (Development|PrintString "Hello"))

(event Custom|OnTrackStarted_Event
  (params (TrackIndex :type Integer))
  (Development|PrintString "Hello"))

(event Input|EnhancedActionEvents|EnhancedInputActionIA_Tap
  (params (ActionValue :type Boolean) (ElapsedSeconds :type Float%20%28double-precision%29) (TriggeredSeconds :type Float%20%28double-precision%29) (InputAction :type Input%20Action%20Object%20Reference :default "/UniversalBeat/Blueprints/IA_Tap.IA_Tap"))
  (bind _returnvalue (Class|UniversalBeatSubsystem|CheckBeatTimingbyLabel (Subsystems|GetUniversalBeatSubsystem) "None"))
  (Development|PrintString (Utilities|String|ToString(Float) _returnvalue)))

(event EventBeginPlay
  (bind _returnvalue (Subsystems|GetUniversalBeatSubsystem))
  (Class|UniversalBeatSubsystem|SetBPM _returnvalue (Variables|Default|GetBPM))
  (Class|UniversalBeatSubsystem|EnableBeatBroadcasting _returnvalue "Sixteenth")
  (Class|UniversalBeatSubsystem|PlaySongbyAsset _returnvalue "/UniversalBeat/Blueprints/BaseSong.BaseSong" false)
  (EventDispatchers|AssignOnSongStarted _returnvalue (delegate Custom|OnSongStarted_Event))
  (EventDispatchers|AssignOnTrackStarted _returnvalue (delegate Custom|OnTrackStarted_Event)))

(fn ConstructionScript)